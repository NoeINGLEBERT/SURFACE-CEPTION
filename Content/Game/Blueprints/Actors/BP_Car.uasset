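; BP_Car is a car actor that lines itself up with the VR player and moves that player onto its child actor's position.
; On BeginPlay it caches the VRPawn and sets its own rotation from the negated camera right vector with Z up.
; After a short delay it teleports the pawn by the camera-to-child-actor offset in X and Y, using a fixed Z height.
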(event `self.ReceiveBeginPlay`
  (bind _player (`self.Player`))
  (bind _camera (`/Game/VRTemplate/Blueprints/VRPawn.Camera` (`self.Player`)))
  (bind (_returnvalue_x _returnvalue_y) (`KismetMathLibrary.BreakVector` (+ (`self.K2_GetActorLocation` _player) (- (`SceneComponent.K2_GetComponentLocation` (`self.ChildActor`)) (`SceneComponent.K2_GetComponentLocation` _camera)))))
  (bind _asvrpawn (cast `/Game/VRTemplate/Blueprints/VRPawn` (`GameplayStatics.GetPlayerPawn` 0)))
  (set `self.Player` _asvrpawn)
  (`self.K2_SetActorRotation` (`KismetMathLibrary.MakeRotFromZX` (0.0 0.0 1.0) (`KismetMathLibrary.NegateVector` (`SceneComponent.GetRightVector` _camera))))
  (`KismetSystemLibrary.Delay` 2.0)
  (`self.K2_SetActorLocation` _player (`KismetMathLibrary.MakeVector` _returnvalue_x _returnvalue_y -5.0) false true))

(fn `UserConstructionScript`)