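; BP_Steer is a grabbable VR steering wheel for the level's BP_Car.
; While held, it slides car and player along the car's right axis according to the player camera's facing, not the wheel angle.
; The wheel follows the motion controller projected onto its plane.
; A gate captures a quaternion offset on each grab or controller change, preserving the wheel's relative angle.
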(event `self.ReceiveBeginPlay`
  (bind _returnvalue (`GameplayStatics.GetActorOfClass` "/Game/Game/Blueprints/Actors/BP_Car.BP_Car_C"))
  (set `self.Vehicle` _returnvalue))

(event `self.ReceiveTick`
  (params (DeltaSeconds :type "Float (single-precision)"))
  (bind _vehicle (`self.Vehicle`))
  (bind _vehicle_2 (`self.Vehicle`))
  (bind _grabcomponent (`self.GrabComponent`))
  (bind _returnvalue (`self.GetActorRightVector` _vehicle_2))
  (bind _returnvalue_2 (`KismetMathLibrary.Normal` (`KismetMathLibrary.ProjectVectorOnToPlane` (- (`SceneComponent.K2_GetComponentLocation` (`/Game/VRTemplate/Blueprints/GrabComponent.MotionControllerRef` _grabcomponent)) (`SceneComponent.K2_GetComponentLocation` (`self.Steer`))) (`SceneComponent.GetUpVector` (`self.Steer`)))))
  (if (`/Game/VRTemplate/Blueprints/GrabComponent.bIsHeld` _grabcomponent)
    (`|ExecutionSequence`
      (:`then_0`
        (for _array_element (`|MakeArray` (`/Game/Game/Blueprints/Actors/BP_Car.Player` _vehicle) _vehicle :!type "Actor Object Reference")
          (`self.K2_SetActorLocation` _array_element (+ (`self.K2_GetActorLocation` _array_element) (* (* _returnvalue (`KismetMathLibrary.Dot_VectorVector` (`SceneComponent.GetForwardVector` (`/Game/VRTemplate/Blueprints/VRPawn.Camera` (`/Game/Game/Blueprints/Actors/BP_Car.Player` _vehicle_2))) _returnvalue)) (* DeltaSeconds 100.0))) false false)))
      (:`then_1`
        (if (not (== (`/Game/VRTemplate/Blueprints/GrabComponent.MotionControllerRef` _grabcomponent) (`self.LazyFix`)))
          (goto _label :!via `Open`)))
      (:`then_2`
        (`/Engine/EditorBlueprintResources/StandardMacros.Gate` true :!label _label
          (:`Exit`
            (`|ExecutionSequence`
              (:`then_0`
                (set `self.Quat` (`KismetMathLibrary.Quat_FindBetweenVectors` _returnvalue_2 (`SceneComponent.GetForwardVector` (`self.Steer`))))
                (set `self.LazyFix` (`/Game/VRTemplate/Blueprints/GrabComponent.MotionControllerRef` _grabcomponent)))
              (:`then_1`
                (goto _label :!via `Close`))))))
      (:`then_3`
        (`SceneComponent.K2_SetWorldRotation` (`self.Steer`) (`KismetMathLibrary.MakeRotFromZX` (`SceneComponent.GetUpVector` (`self.Steer`)) (`KismetMathLibrary.Quat_RotateVector` (`self.Quat`) _returnvalue_2)) false false)))
    (else
      (goto _label :!via `Open`))))

(fn `UserConstructionScript`)