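; BP_Phone is a grabbable phone actor for motion controllers that reorients itself by holding hand and tracks a touching fingertip.
; Each Tick checks GrabComponent's controller, using a Gate to flip the phone's forward vector once on a right-hand grab, re-arming when released or held otherwise.
; Touch stores the fingertip from any controller other than the holding one.
; Debug prints report touches, snaps and the fingertip's world location every frame.
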(event `/Game/Game/Blueprints/Interfaces/BPI_Phone.Touch`
  (params (MotionController :type "MotionControllerComponent Object Reference") (FingerTip :type "SceneComponent Object Reference"))
  (if (!= MotionController (`/Game/VRTemplate/Blueprints/GrabComponent.MotionControllerRef` (`self.GrabComponent`)))
    (bind _output_get (set `self.FingerRef` FingerTip))
    (`/Engine/EditorBlueprintResources/StandardMacros.IsValid` _output_get
      (:`Is Valid`
        (`KismetSystemLibrary.PrintString` "IN" true true (struct :`G` 1.0 :`A` 1.0)))
      (:`Is Not Valid`
        (`KismetSystemLibrary.PrintString` "OUT" true true (struct :`R` 1.0 :`A` 1.0))))))

(event `self.ReceiveTick`
  (params (DeltaSeconds :type "Float (single-precision)"))
  (bind _phone (`self.Phone`))
  (`|ExecutionSequence`
    (:`then_0`
      (bind _motioncontrollerref (`/Game/VRTemplate/Blueprints/GrabComponent.MotionControllerRef` (`self.GrabComponent`))
        (:`then`
          (if (== (`MotionControllerComponent.MotionSource` _motioncontrollerref) "Right")
            (`/Engine/EditorBlueprintResources/StandardMacros.Gate` true :!label _label
              (:`Exit`
                (`|ExecutionSequence`
                  (:`then_0`
                    (`KismetSystemLibrary.PrintString` "SNAP" true true (struct :`R` 1.0 :`B` 1.0 :`A` 1.0))
                    (`SceneComponent.K2_SetRelativeRotation` _phone (`KismetMathLibrary.MakeRotFromZX` (`SceneComponent.GetUpVector` _phone) (`KismetMathLibrary.NegateVector` (`SceneComponent.GetForwardVector` _phone))) false false))
                  (:`then_1`
                    (goto _label :!via `Close`)))))
            (else
              (goto _label :!via `Open`))))
        (:`else`
          (goto _label :!via `Open`))))
    (:`then_1`
      (`KismetSystemLibrary.PrintString` (`KismetStringLibrary.Conv_VectorToString` (`SceneComponent.K2_GetComponentLocation` (`self.FingerRef`))) true true (struct :`B` 1.0 :`A` 1.0)))))

(fn `UserConstructionScript`)