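; BP_CarPlace is a grabbable spot, apparently a car seat, that snaps the VR pawn into place when held.
; Tick polls the grab component, using a gate reopened on release so the snap runs once per grab.
; The snap sets a fixed pawn rotation, then teleports it so the camera lines up horizontally with the child actor, with height taken slightly below this actor's origin.
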(event `self.ReceiveBeginPlay`
  (bind _asvrpawn (cast `/Game/VRTemplate/Blueprints/VRPawn` (`GameplayStatics.GetPlayerPawn` 0)))
  (set `self.As VRPawn` _asvrpawn))

(event `self.ReceiveTick`
  (params (DeltaSeconds :type "Float (single-precision)"))
  (bind (_returnvalue_x _returnvalue_y _returnvalue_z) (`KismetMathLibrary.BreakVector` (`self.K2_GetActorLocation`)))
  (bind _as_vrpawn (`self.As VRPawn`))
  (bind (_returnvalue_x_2 _returnvalue_y_2) (`KismetMathLibrary.BreakVector` (+ (`self.K2_GetActorLocation` _as_vrpawn) (- (`SceneComponent.K2_GetComponentLocation` (`self.ChildActor`)) (`SceneComponent.K2_GetComponentLocation` (`/Game/VRTemplate/Blueprints/VRPawn.Camera` (`self.As VRPawn`)))))))
  (if (`/Game/VRTemplate/Blueprints/GrabComponent.bIsHeld` (`self.GrabComponent`))
    (`/Engine/EditorBlueprintResources/StandardMacros.Gate` true :!label _label
      (:`Exit`
        (`|ExecutionSequence`
          (:`then_0`
            (`self.K2_SetActorRelativeRotation` _as_vrpawn (struct :`Yaw` 90.0) false false)
            (`self.K2_SetActorLocation` _as_vrpawn (`KismetMathLibrary.MakeVector` _returnvalue_x_2 _returnvalue_y_2 (- _returnvalue_z 5.0)) false true))
          (:`then_1`
            (goto _label :!via `Close`)))))
    (else
      (goto _label :!via `Open`))))

(fn `UserConstructionScript`)